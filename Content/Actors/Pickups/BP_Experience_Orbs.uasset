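; Experience orb pickup that pops out with a random impulse on spawn and becomes collectible after a short random delay.
; An overlap message stores the initiator and toggles Tick, which lerps the Cone component toward that actor once collectible.
; ItemCollected runs once, sending the XP value to the collector through a GrantXP message and destroying the orb.
; Its own ApplyDamage and GrantXP functions are empty.
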(event `self.ReceiveBeginPlay`
  (bind _returnvalue (`KismetMathLibrary.RandomFloatInRange` -300.0 300.0))
  (bind _cone (`self.Cone`))
  (`PrimitiveComponent.AddVelocityChangeImpulseAtLocation` _cone (`KismetMathLibrary.MakeVector` _returnvalue _returnvalue (`KismetMathLibrary.RandomFloatInRange` 600.0 1000.0)) (`SceneComponent.RelativeLocation` _cone) "None")
  (`KismetSystemLibrary.Delay` (`KismetMathLibrary.RandomFloatInRange` 0.5 1.5))
  (set `self.Is Collectible` true))

(event `self.ReceiveTick`
  (params (DeltaSeconds :type "Float (single-precision)"))
  (bind _cone (`self.Cone`))
  (bind (_returnvalue_location _returnvalue_rotation _returnvalue_scale) (`KismetMathLibrary.BreakTransform` (`SceneComponent.GetRelativeTransform` _cone)))
  (bind (_returnvalue_location_2 _returnvalue_rotation_2) (`KismetMathLibrary.BreakTransform` (`self.GetTransform` (`self.Overlap Initiator`))))
  (bind (_returnvalue_location_3 _returnvalue_rotation_3) (`KismetMathLibrary.BreakTransform` (`KismetMathLibrary.TLerp` (`KismetMathLibrary.MakeTransform` _returnvalue_location _returnvalue_rotation _returnvalue_scale) (`KismetMathLibrary.MakeTransform` _returnvalue_location_2 _returnvalue_rotation_2 _returnvalue_scale) 0.05)))
  (if (`self.Is Collectible`)
    (`SceneComponent.K2_SetWorldTransform` _cone (`KismetMathLibrary.MakeTransform` _returnvalue_location_3 _returnvalue_rotation_3 _returnvalue_scale) false false)))

(event `/Game/Gameplay_Actors_Interface.Actor Was Overlapped`
  (params (`Overlap Initiator` :type "Actor Object Reference") (`Overlap State` :type Boolean) (`Radius Triggered By` :type "SphereComponent Object Reference"))
  (set `self.Overlap Initiator` `Overlap Initiator`)
  (`self.SetActorTickEnabled` `Overlap State`))

(fn `Apply Damage`
  (params (`Damage To Apply` :type "Float (double-precision)"))
  (returns (`Damaged Actor` :type "Actor Object Reference"))
  (return null))

(fn `Grant XP`
  (params (`XP To Grant` :type "Float (double-precision)"))
  (returns (`Xp Granted To` :type "Actor Object Reference"))
  (return null))

(fn `Item Collected`
  (params (Collector :type "Actor Object Reference"))
  (returns (`Item Collected` :type "Actor Object Reference"))
  (`/Engine/EditorBlueprintResources/StandardMacros.DoOnce` false
    (:`Completed`
      (message `/Game/Gameplay_Actors_Interface.Grant XP` Collector (`self.Xp Value`))
      (`self.K2_DestroyActor`)
      (return self))))

(fn `UserConstructionScript`)