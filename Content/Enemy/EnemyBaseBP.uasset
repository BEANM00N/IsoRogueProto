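; Base enemy Blueprint with a laser sight and a minigun secondary attack.
; Tick traces from the laser socket to set the red beam's end and the shared impact point, and derives a base rotator from velocity while moving.
; A timer, looping when fully automatic, spawns projectiles and muzzle flashes at the barrel, aimed at that point with random cone spread, and clears once CanSee is false.
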(event `self.ReceiveBeginPlay`
  (bind _mesh (`self.Mesh`))
  (bind (_returnvalue_location _returnvalue_rotation) (`KismetMathLibrary.BreakTransform` (`SceneComponent.GetSocketTransform` _mesh "Laser Sight" "RTS_World")))
  (bind _returnvalue (`NiagaraFunctionLibrary.SpawnSystemAttached` "/Game/Player/LaserPointerRed.LaserPointerRed" _mesh "Laser Sight" (0.0 0.0 0.0) _returnvalue_rotation "KeepRelativeOffset"))
  (set `self.LaserPointer` _returnvalue)
  (add `self.FireSecondary` (delegate `Fire Secondary`)))

(event `Fire Secondary`
  (bind _returnvalue (`KismetSystemLibrary.K2_SetTimer` null "FireSecondaryFunction" 0.05 (`self.FullyAutomatic?`)))
  (set `self.FireSecondaryTimer` _returnvalue))

(event `self.ReceiveTick`
  (params (DeltaSeconds :type "Float (single-precision)"))
  (bind (_returnvalue_location _returnvalue_rotation) (`KismetMathLibrary.BreakTransform` (`SceneComponent.GetSocketTransform` (`self.Mesh`) "Laser Sight" "RTS_World")))
  (bind _velocity (`MovementComponent.Velocity` (`self.CharacterMovement`)))
  (if (not (== _velocity (0.0 0.0 0.0)))
    (set `self.BaseRotator` (`KismetMathLibrary.MakeRotFromX` _velocity)))
  (bind _outhit (`KismetSystemLibrary.LineTraceSingle` _returnvalue_location (+ _returnvalue_location (* (`KismetMathLibrary.GetForwardVector` _returnvalue_rotation) 10000.0)) "TraceTypeQuery2"))
  (bind _laserpointer (`self.LaserPointer`)
    (:`then`
      (bind (_bblockinghit _binitialoverlap _time _distance _location _impactpoint _normal _impactnormal _physmat _hitactor _hitcomponent _hitbonename _bonename _hititem _elementindex _faceindex _tracestart _traceend) (`GameplayStatics.BreakHitResult` _outhit))
      (if _bblockinghit
        (`FXSystemComponent.SetVectorParameter` _laserpointer "Beam End" _impactpoint)
        (set `self.Impact Point` _impactpoint)
        (else
          (`FXSystemComponent.SetVectorParameter` _laserpointer "Beam End" _traceend)
          (set `self.Impact Point` _traceend))))
    (:`else`)))

(fn `Align to Laser`
  (params (Start :type "Vector Structure (by ref)") (Target :type "Vector Structure (by ref)") (ConeHalfAngleInDegrees :type "Float (single-precision)"))
  (returns (ReturnValue :type "Rotator Structure"))
  (bind _returnvalue (`KismetMathLibrary.GetForwardVector` (`KismetMathLibrary.FindLookAtRotation` Start Target)))
  (return (`KismetMathLibrary.MakeRotFromX` (+ _returnvalue (`KismetMathLibrary.RandomUnitVectorInConeInDegrees` _returnvalue ConeHalfAngleInDegrees)))))

(fn `FireSecondaryFunction`
  (bind _returnvalue_location (`KismetMathLibrary.BreakTransform` (`SceneComponent.GetSocketTransform` (`self.Minigun`) "BARREL" "RTS_World")))
  (bind _returnvalue (`self.Align to Laser` _returnvalue_location (`self.Impact Point`) 5.0))
  (`|SpawnActorFromClass` "/Game/Player/Projectiles/SecondaryProjectile.SecondaryProjectile_C" (`KismetMathLibrary.MakeTransform` _returnvalue_location _returnvalue) "Undefined" "MultiplyWithRoot" null null)
  (`NiagaraFunctionLibrary.SpawnSystemAttachedWithParams` (make `FXSystemSpawnParameters` null "/Game/VFX/MuzzleFX/FX/NiagaraSystems/NS_AR_Muzzleflash_2_ONCE.NS_AR_Muzzleflash_2_ONCE" (0.0 0.0 0.0) (struct) (`KismetMathLibrary.Conv_DoubleToVector` 0.4) (`self.Minigun`) "BARREL" "KeepRelativeOffset"))
  (if (not (`self.CanSee`))
    (`KismetSystemLibrary.K2_ClearAndInvalidateTimerHandle` (`self.FireSecondaryTimer`)))
  (return))

(fn `UserConstructionScript`)