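; BP_GM_Panzer is a game mode Blueprint with a SpawnPlayer routine for giving joining players a character.
; SpawnPlayer records the controller, gathers all PlayerStart actors, spawns a PlayerCharacter at a random one's location and possesses it.
; It then prints the new character's owner name for debugging.
; PostLogin is empty and the SpawnPlayer call in the event graph is disconnected, so this graph never triggers spawning.
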(event `self.K2_PostLogin`
  (params (NewPlayer :type "PlayerController Object Reference")))

(fn `Spawn Player`
  (params (Controller :type "PlayerController Object Reference"))
  (`KismetArrayLibrary.Array_Add` (`self.All Player Controllers`) Controller)
  (bind _outactors (`GameplayStatics.GetAllActorsOfClass` "/Script/Engine.PlayerStart"))
  (set `self.PlayerSpawns` _outactors)
  (bind _returnvalue (`|SpawnActorFromClass` "/Game/Player/PlayerCharacter.PlayerCharacter_C" (`KismetMathLibrary.MakeTransform` (`self.K2_GetActorLocation` (`KismetArrayLibrary.Array_Random` (`self.PlayerSpawns`)))) "Undefined" "MultiplyWithRoot" null null))
  (`Controller.Possess` Controller _returnvalue)
  (`KismetSystemLibrary.PrintString` (`KismetSystemLibrary.GetDisplayName` (`self.GetOwner` _returnvalue)) true true (struct :`R` 1.0 :`G` 0.269289 :`A` 1.0) 12.0))

(fn `UserConstructionScript`)