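; Player controller for the Panzer game mode that requests its player's spawn when play begins.
; On BeginPlay, the local controller switches input to game-only and calls SR_SpawnPlayer, which casts the game mode to BP_GM_Panzer and passes itself to SpawnPlayer.
; Disconnected leftover nodes would set game-and-UI input or add a UI_Card_Holder widget to the viewport, but never run.
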(event `self.ReceiveBeginPlay`
  (if (`self.IsLocalPlayerController`)
    (`WidgetBlueprintLibrary.SetInputMode_GameOnly` self)
    (`self.SR_SpawnPlayer`)))

(event `SR_SpawnPlayer`
  (bind _asbp_gm_panzer (cast `/Game/Player/Core/BP_GM_Panzer` (`GameplayStatics.GetGameMode`)))
  (`/Game/Player/Core/BP_GM_Panzer.Spawn Player` _asbp_gm_panzer self))

(fn `UserConstructionScript`)