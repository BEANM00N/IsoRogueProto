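; Base secondary weapon module, an auto-targeting turret that aims at the nearest MinionBase actor and fires MG_Shot_BASE projectiles at it.
; LockToTarget rotates the mesh and calls FireOnTarget, which starts a looping timer that spawns shots from the TurretBarrel socket.
; An empty magazine stops firing and schedules a timed reload.
; Upgrades run by function name from a data asset, such as DamageUpgrade, which triples damage.
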(event `/Game/Player/Modules/Module_Interface.Damage Upgrade`
  (bind _weapon_damage (`self.Weapon Damage`))
  (`KismetSystemLibrary.PrintString` (`KismetStringLibrary.Conv_DoubleToString` _weapon_damage) true true (struct :`R` 0.08091 :`G` 0.459097 :`B` 1.0 :`A` 1.0) 5.0)
  (`|VariableSetRef` _weapon_damage (* _weapon_damage 3.0))
  (`KismetSystemLibrary.PrintString` (`KismetStringLibrary.Conv_DoubleToString` _weapon_damage) true true (struct :`R` 1.0 :`G` 0.155166 :`A` 1.0) 5.0))

(event `/Game/Player/Modules/Module_Interface.Trigger Upgrade`
  (params (`Data Asset Reference` :type "/Game/UI/HUD/Cards/CardDataAssets/BP_DA_Card_Base Object Reference"))
  (`KismetSystemLibrary.K2_SetTimer` null (`/Game/UI/HUD/Cards/CardDataAssets/BP_DA_Card_Base.UpgradeFunctionName` `Data Asset Reference`) 0.01))

(fn `Activate Module`
  (params (`Player Reference` :type "/Game/Player/PlayerCharacter Object Reference"))
  (returns (`Module Activated` :type "Actor Object Reference"))
  (set `self.Player Reference` `Player Reference`)
  (return self))

(fn `Fire On Target`
  (if (not (or (`KismetSystemLibrary.K2_IsValidTimerHandle` (`self.Firing Timer`)) (`self.Reloading`)))
    (`self.Fire Weapon`)
    (bind _returnvalue (`KismetSystemLibrary.K2_SetTimer` null "Fire Weapon" (`self.Fire Rate`) true))
    (set `self.Firing Timer` _returnvalue)
    (return)))

(fn `Fire Weapon`
  (bind (_returnvalue_location _returnvalue_rotation) (`KismetMathLibrary.BreakTransform` (`SceneComponent.GetSocketTransform` (`self.Mesh`) "TurretBarrel" "RTS_World")))
  (bind _result (`/Engine/EditorBlueprintResources/StandardMacros.DecrementInt` (`self.Current Ammo`))
    (:`  `
      (if (<= _result 0)
        (set `self.Reloading` true)
        (`KismetSystemLibrary.K2_ClearAndInvalidateTimerHandle` (`self.Firing Timer`))
        (bind _returnvalue (`KismetSystemLibrary.K2_SetTimer` null "Reload" (`self.Reload Time`)))
        (set `self.Reload Timer` _returnvalue)
        (`KismetSystemLibrary.PrintString` "Reload" true true (struct :`R` 1.0 :`B` 0.005134 :`A` 1.0) 10.0)
        (else
          (`KismetSystemLibrary.PrintString` (`KismetTextLibrary.Conv_TextToString` (`|FormatText` "{Current Ammo}/{Mag Size}" _result (`self.Magazine Size`))) true true (struct :`R` 1.0 :`G` 0.309979 :`B` 0.642185 :`A` 1.0) (`self.Fire Rate`))
          (`|SpawnActorFromClass` "/Game/Player/Projectiles/MG_Shot_BASE.MG_Shot_BASE_C" (`KismetMathLibrary.MakeTransform` _returnvalue_location _returnvalue_rotation) "Undefined" "MultiplyWithRoot" null (`self.Weapon Damage`) "Enemy" null)
          (return))))))

(fn `Lock To Target`
  (returns (Reference :type "Actor Object Reference"))
  (bind _mesh (`self.Mesh`))
  (bind _outactors (`GameplayStatics.GetAllActorsOfClass` "/Game/Enemy/MinionBase.MinionBase_C"))
  (if (not (`KismetArrayLibrary.Array_IsEmpty` _outactors))
    (bind (_distance _returnvalue) (`GameplayStatics.FindNearestActor` (`SceneComponent.K2_GetComponentLocation` (`self.DefaultSceneRoot`)) _outactors))
    (set `self.Targeted Actor` _returnvalue)
    (bind (_returnvalue_roll _returnvalue_pitch _returnvalue_yaw) (`KismetMathLibrary.BreakRotator` (`KismetMathLibrary.FindLookAtRotation` (`SceneComponent.K2_GetComponentLocation` _mesh) (`self.K2_GetActorLocation` _returnvalue))))
    (`SceneComponent.K2_SetWorldRotation` _mesh (`KismetMathLibrary.MakeRotator` _returnvalue_roll _returnvalue_pitch (- _returnvalue_yaw 90.0)) false false))
  (`self.Targeted Actor`
    (:`then`
      (`self.Fire On Target`)
      (return self))
    (:`else`
      (`KismetSystemLibrary.K2_ClearAndInvalidateTimerHandle` (`self.Firing Timer`)))))

(fn `Reload`
  (`|VariableSetRef` (`self.Current Ammo`) (`self.Magazine Size`))
  (set `self.Reloading` false)
  (`KismetSystemLibrary.PrintString` "Reloaded")
  (return))

(fn `Trigger`
  (params (Player :type "/Game/Player/PlayerCharacter Object Reference") (ValidInput :type Boolean))
  (returns (Module :type "Actor Object Reference"))
  (return null))

(fn `UserConstructionScript`
  (`|VariableSetRef` (`self.Current Ammo`) (`self.Magazine Size`)))