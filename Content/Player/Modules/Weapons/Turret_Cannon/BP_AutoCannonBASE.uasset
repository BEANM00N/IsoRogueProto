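; Base auto-cannon weapon module for the player, adding magazine-fed automatic fire and timed reloads to its parent weapon class.
; Trigger starts Fire after a can-fire check, and releasing it clears the looping fire timer that Fire re-arms after each parent shot.
; An empty magazine blocks firing and starts a timed Reload, which refills it and resumes firing if input is held.
; Ammo count and reload wheel are pushed to the player HUD.
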(fn `Activate Module`
  (params (`Player Reference` :type "/Game/Player/PlayerCharacter Object Reference"))
  (returns (`Module Activated` :type "Actor Object Reference"))
  (bind _magazine_ammo (`self.Magazine Ammo`))
  (bind _magazine_max_capacity (`self.Magazine Max Capacity`))
  (bind _output_get (set `self.Player` `Player Reference`))
  (`|VariableSetRef` _magazine_ammo _magazine_max_capacity)
  (`/Game/Player/PlayerHUD.Update Ammunition` (`/Game/Player/PlayerCharacter.PlayerHUD` _output_get) _magazine_ammo _magazine_max_capacity)
  (return self))

(fn `Decrease Ammo in Mag`
  (bind _result (`/Engine/EditorBlueprintResources/StandardMacros.DecrementInt` (`self.Magazine Ammo`))
    (:`  `
      (`/Game/Player/PlayerHUD.Update Ammunition` (`/Game/Player/PlayerCharacter.PlayerHUD` (`self.Player`)) _result (`self.Magazine Max Capacity`)))))

(fn `Fire`
  (bind _reload_timer (`self.Reload Timer`))
  (if (<= (`self.Magazine Ammo`) 0)
    (`KismetSystemLibrary.K2_ClearAndInvalidateTimerHandle` (`self.Firing Timer`))
    (set `self.Can Fire?` false)
    (bind _returnvalue (`KismetSystemLibrary.K2_SetTimer` null "Reload" _reload_timer))
    (`/Game/Player/PlayerHUD.Activate Reload Wheel` (`/Game/Player/PlayerCharacter.PlayerHUD` (`self.Player`)) _returnvalue _reload_timer)
    (else
      (`parent.Fire`)
      (`self.Decrease Ammo in Mag`)
      (bind _returnvalue_2 (`KismetSystemLibrary.K2_SetTimer` null "Fire" (`self.Fire Rate`) true 0.01))
      (set `self.Firing Timer` _returnvalue_2)))
  (return))

(fn `Reload`
  (bind _magazine_ammo (`self.Magazine Ammo`))
  (bind _magazine_max_capacity (`self.Magazine Max Capacity`))
  (set `self.Can Fire?` true)
  (`|VariableSetRef` _magazine_ammo _magazine_max_capacity)
  (`/Game/Player/PlayerHUD.Update Ammunition` (`/Game/Player/PlayerCharacter.PlayerHUD` (`self.Player`)) _magazine_ammo _magazine_max_capacity)
  (if (`self.Valid Input`)
    (`self.Fire`)))

(fn `Trigger`
  (params (Player :type "/Game/Player/PlayerCharacter Object Reference") (ValidInput :type Boolean))
  (returns (Module :type "Actor Object Reference"))
  (set `self.Player` Player)
  (set `self.Valid Input` ValidInput)
  (if ValidInput
    (bind _output_get (`self.Can Fire Check`))
    (if _output_get
      (`self.Fire`)
      (return self))
    (else
      (`KismetSystemLibrary.K2_ClearAndInvalidateTimerHandle` (`self.Firing Timer`)))))

(fn `UserConstructionScript`
  (`parent.UserConstructionScript`))