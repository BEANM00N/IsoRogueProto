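; Medium autocannon player turret module that overrides projectile spawning to alternate fire between two barrels, without calling the parent version.
; Each shot spawns a Cannon_Shot_BASE at the current barrel socket, aimed at the impact point and given damage and penetration values.
; It then flips the barrel index for the next shot.
; Muzzle FX always attaches to ProjectileSocket rather than the firing barrel's socket, and a debug print logs every shot.
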(fn `Spawn Projectile`
  (bind _barrel_to_fire_from (`self.Barrel To Fire From`))
  (bind _barrel_to_fire_from_2 (`self.Barrel To Fire From`))
  (bind _returnvalue (`KismetMathLibrary.SelectInt` _barrel_to_fire_from 1 (== _barrel_to_fire_from 0)))
  (bind _output (`|GetArrayItem` (`self.In Socket Name`) _returnvalue))
  (bind _returnvalue_2 (`SceneComponent.GetSocketLocation` (`self.Mesh`) _output))
  (`KismetSystemLibrary.PrintString` (`KismetTextLibrary.Conv_TextToString` (`|FormatText` "Firing {Name}  \n{Val}" _output _returnvalue)) true true (struct :`R` 1.0 :`G` 0.168426 :`B` 0.338834 :`A` 1.0))
  (`|SpawnActorFromClass` "/Game/Player/Projectiles/Cannon_Shot_BASE.Cannon_Shot_BASE_C" (`KismetMathLibrary.MakeTransform` _returnvalue_2 (`KismetMathLibrary.FindLookAtRotation` _returnvalue_2 (`self.Impact Point`))) "Undefined" "MultiplyWithRoot" (`self.Player`) (`self.Damage`) (`self.Gun Penetration`) null)
  (`NiagaraFunctionLibrary.SpawnSystemAttachedWithParams` (make `FXSystemSpawnParameters` null (`self.Muzzle FX`) (0.0 0.0 0.0) (struct) (`self.Muzzle FX Scale`) (`self.Mesh`) (`self.ProjectileSocket`) "KeepRelativeOffset"))
  (if (> _barrel_to_fire_from_2 0)
    (`|VariableSetRef` _barrel_to_fire_from_2)
    (else
      (`/Engine/EditorBlueprintResources/StandardMacros.IncrementInt` _barrel_to_fire_from_2
        (:`  `
          _))))
  (return))

(fn `UserConstructionScript`
  (`parent.UserConstructionScript`))