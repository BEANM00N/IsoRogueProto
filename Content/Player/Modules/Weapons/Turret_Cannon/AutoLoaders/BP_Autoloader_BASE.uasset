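; Base autoloader cannon module for the player's turret, firing repeatedly from a limited magazine while input is held.
; Trigger starts firing when ammo is loaded and no intra-shot timer runs; a looping timer then calls Cycle Gun for follow-up shots.
; An empty magazine starts a reload timer, and Reload refills it and resumes firing if input is valid.
; The weapon widget shows ammo count and reload wheels.
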(event `self.ReceiveBeginPlay`
  (`parent.ReceiveBeginPlay`))

(fn `Activate Module`
  (params (`Player Reference` :type "/Game/Player/PlayerCharacter Object Reference"))
  (returns (`Module Activated` :type "Actor Object Reference"))
  (set `self.Player` `Player Reference`)
  (`/Game/Player/UI/Widgets/RadialProgressBar/UMG_Reload_Wheel.Update Ammunition` (`self.Weapon Widget`) (`self.Rounds Loaded`) (`self.Max Rounds `))
  (return self))

(fn `Cycle Gun`
  (bind _weapon_widget (`self.Weapon Widget`))
  (if (and (`self.Valid Input`) (`self.Has Ammo?`))
    ;[1 1 1] Next Shell is Loaded
    (`self.Fire`)
    (else
      ;[1 1 1] Gun's empty, Reload Canister
      (`KismetSystemLibrary.K2_ClearAndInvalidateTimerHandle` (`self.Intra Shot Timer`))
      (if (not (`self.Has Ammo?`))
        (bind _returnvalue (`KismetSystemLibrary.K2_SetTimer` null "Reload" (`self.Reload Timer`)))
        (bind _output_get (set `self.Reload Timer Handle` _returnvalue))
        (`/Game/Player/UI/Widgets/RadialProgressBar/UMG_Reload_Wheel.Activate Reload Wheel` _weapon_widget _output_get (`self.Reload Timer`))
        (`/Game/Player/UI/Widgets/RadialProgressBar/UMG_Reload_Wheel.Update Ammunition` _weapon_widget 0 0)))))

(fn `Fire`
  (bind _weapon_widget (`self.Weapon Widget`))
  (`parent.Fire`)
  (bind _result (`/Engine/EditorBlueprintResources/StandardMacros.DecrementInt` (`self.Rounds Loaded`))
    (:`  `
      (if (< _result 1)
        (`KismetSystemLibrary.PrintString` "No Ammo")
        (set `self.Has Ammo?` false)
        (`self.Cycle Gun`)
        (else
          (`/Game/Player/UI/Widgets/RadialProgressBar/UMG_Reload_Wheel.Update Ammunition` (`self.Weapon Widget`) (`self.Rounds Loaded`) (`self.Max Rounds `))
          (bind _returnvalue (`KismetSystemLibrary.K2_SetTimer` null "Cycle Gun" (`self.Intra-Shot Reload`) true))
          (bind _output_get (set `self.Intra Shot Timer` _returnvalue))
          (`/Game/Player/UI/Widgets/RadialProgressBar/UMG_Reload_Wheel.Activate Reload Wheel` _weapon_widget _output_get (`self.Intra-Shot Reload`))
          (`/Game/Player/UI/Widgets/RadialProgressBar/UMG_Reload_Wheel.Update Ammunition` _weapon_widget (`self.Rounds Loaded`) (`self.Max Rounds `)))))))

(fn `Reload`
  (`parent.Reload`)
  (set `self.Rounds Loaded` (`self.Max Rounds `))
  (set `self.Has Ammo?` true)
  (`/Game/Player/UI/Widgets/RadialProgressBar/UMG_Reload_Wheel.Update Ammunition` (`self.Weapon Widget`) (`self.Rounds Loaded`) (`self.Max Rounds `))
  (if (`self.Valid Input`)
    (`self.Fire`)))

(fn `Trigger`
  (params (Player :type "/Game/Player/PlayerCharacter Object Reference") (ValidInput :type Boolean))
  (returns (Module :type "Actor Object Reference"))
  (set `self.Player` Player)
  (set `self.Valid Input` ValidInput)
  ;[0.7911 0.5624 1] How To make True = False returns on an AND to avoid "Multi-Branches"
  (if (and (`self.Has Ammo?`) (`self.Valid Input`) (not (`KismetSystemLibrary.K2_IsValidTimerHandle` (`self.Intra Shot Timer`))))
    (`self.Fire`)
    (return self)))

(fn `UserConstructionScript`
  (`parent.UserConstructionScript`))