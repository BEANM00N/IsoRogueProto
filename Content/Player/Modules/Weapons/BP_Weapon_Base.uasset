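; Base player weapon module, the "Main Cannon", that fires projectiles toward the player's aim impact point with random cone spread.
; Trigger calls Fire, which spawns the projectile, muzzle FX, camera shake and an ejected shell casing.
; A timer drives Reload and the HUD reload wheel, then re-triggers while input stays valid for automatic fire.
; LockToTarget toggles an auto-aim flag, but the rotation code using it is disconnected.
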(event `self.ReceiveBeginPlay`
  (set `self.Can Fire?` true))

(fn `Activate Module`
  (params (`Player Reference` :type "/Game/Player/PlayerCharacter Object Reference"))
  (returns (`Module Activated` :type "Actor Object Reference"))
  (set `self.Player` `Player Reference`)
  (`KismetSystemLibrary.PrintString` "Main Cannon Online" true true (struct :`R` 1.0 :`G` 0.260123 :`B` 0.694879 :`A` 1.0) 7.6)
  (return self))

(fn `Align to Laser`
  (params (Player :type "/Game/Player/PlayerCharacter Object Reference"))
  (returns (ReturnValue :type "Rotator Structure") (`Socket Location` :type "Vector Structure"))
  (bind _returnvalue_location (`KismetMathLibrary.BreakTransform` (`SceneComponent.GetSocketTransform` (`self.Mesh`) (`self.ProjectileSocket`) "RTS_World")))
  (bind _returnvalue (`KismetMathLibrary.GetForwardVector` (`KismetMathLibrary.FindLookAtRotation` _returnvalue_location (`/Game/Player/PlayerCharacter.Impact Point` Player))))
  (return (`KismetMathLibrary.MakeRotFromX` (+ _returnvalue (`KismetMathLibrary.RandomUnitVectorInConeInDegrees` _returnvalue (`self.Weapon Accuracy`)))) _returnvalue_location))

(fn `Can Fire Check`
  (returns (Output_Get :type Boolean))
  (bind _can_fire_ (`self.Can Fire?`))
  (`KismetSystemLibrary.PrintString` (`KismetStringLibrary.Conv_BoolToString` _can_fire_))
  (return _can_fire_))

(fn `Fire`
  (bind _output_get (`self.Can Fire Check`))
  (if _output_get
    (bind (_returnvalue _socket_location) (`self.Align to Laser` (`self.Player`)))
    (`self.Spawn Projectile` _returnvalue _socket_location)
    (`self.Play Firing Animations`)
    (return)))

(fn `Lock To Target`
  (returns (Reference :type "Actor Object Reference"))
  (`/Engine/EditorBlueprintResources/StandardMacros.FlipFlop`
    (:`A`
      (set `self.Auto Aim Enabled?` true))
    (:`B`
      (set `self.Auto Aim Enabled?` false)))
  (return null))

(fn `Play Firing Animations`
  (bind _returnvalue (`KismetMathLibrary.RandomFloatInRange` 150.0 300.0))
  (bind (_returnvalue_location _returnvalue_rotation) (`KismetMathLibrary.BreakTransform` (`SceneComponent.GetSocketTransform` (`self.Mesh`) "EjectionPort" "RTS_World")))
  (`GameplayStatics.PlayWorldCameraShake` "/Game/Player/Camera_Shakes/Camera_Shake_Test.Camera_Shake_Test_C" (`SceneComponent.K2_GetComponentLocation` (`/Game/Player/PlayerCharacter.CineCamera` (`self.Player`))) 100.0 100.0)
  (bind _returnvalue_2 (`|SpawnActorFromClass` "/Game/Player/Modules/Weapons/Shells/Shell_Casing_BASE.Shell_Casing_BASE_C" (`KismetMathLibrary.MakeTransform` _returnvalue_location _returnvalue_rotation (0.6 0.6 0.6)) "Undefined" "MultiplyWithRoot" null null))
  (`PrimitiveComponent.AddVelocityChangeImpulseAtLocation` (`/Game/Player/Modules/Weapons/Shells/Shell_Casing_BASE.Shell_Mesh` _returnvalue_2) (`KismetMathLibrary.MakeVector` _returnvalue _returnvalue (`KismetMathLibrary.RandomFloatInRange` 760.0 1200.0)) _returnvalue_location "None")
  (return))

(fn `Reload`
  (set `self.Can Fire?` true)
  (`KismetSystemLibrary.K2_ClearAndInvalidateTimerHandle` (`self.FireTimer`))
  (`KismetSystemLibrary.PrintString` "Reloaded!")
  (if (`self.Valid Input`)
    (`self.Trigger` (`self.Player`) (`self.Valid Input`))
    (return)))

(fn `Spawn Projectile`
  (params (SpawnTransform_Rotation :type "Rotator Structure") (SpawnTransform_Location :type "Vector Structure"))
  (`|SpawnActorFromClass` "/Game/Player/Projectiles/PrimaryProjectile.PrimaryProjectile_C" (`KismetMathLibrary.MakeTransform` SpawnTransform_Location SpawnTransform_Rotation) "Undefined" "MultiplyWithRoot" null (`self.Damage`) null)
  (`NiagaraFunctionLibrary.SpawnSystemAttachedWithParams` (make `FXSystemSpawnParameters` null (`self.Muzzle FX`) (0.0 0.0 0.0) (struct) (`self.Muzzle FX Scale`) (`self.Mesh`) (`self.ProjectileSocket`) "KeepRelativeOffset"))
  (return))

(fn `Trigger`
  (params (Player :type "/Game/Player/PlayerCharacter Object Reference") (ValidInput :type Boolean))
  (returns (Module :type "Actor Object Reference"))
  ;[0 0 0] Weapon Triggered
  (bind _output_get (set `self.Valid Input` ValidInput))
  (if _output_get
    (`self.Fire`)
    (if (`self.Can Fire?`)
      (bind _returnvalue (`KismetSystemLibrary.K2_SetTimer` null "Reload" (`self.Reload Timer`)))
      (set `self.Can Fire?` false)
      (bind _output_get_2 (set `self.FireTimer` _returnvalue))
      (`/Game/Player/PlayerHUD.Activate Reload Wheel` (`/Game/Player/PlayerCharacter.PlayerHUD` (`self.Player`)) _output_get_2 (`self.Reload Timer`))
      (return self))))

(fn `UserConstructionScript`)